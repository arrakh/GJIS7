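; BPC_Interactables is a Blueprint component that handles interaction and overlap notifications for interactable objects.
; Interact, StartInteract, EndInteract, StartOverlap and EndOverlap each relay to a matching event dispatcher, leaving the response to whatever binds to it.
; StartOverlap and EndOverlap also toggle Render Custom Depth on a referenced component, the usual hook for an outline highlight.
; BeginPlay only runs a short delay with nothing after it.
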(event EventBeginPlay
  (Utilities|FlowControl|Delay 0.1))

(event EventInteract
  (params (PlayerRef :type BP%20Player%20Object%20Reference))
  (Default|CallOnInteract))

(fn EndInteract
  (Default|CallOnEndIInteract)
  (return false))

(fn EndOverlap
  (Rendering|SetRenderCustomDepth (Variables|Default|GetComponent) false)
  (Default|CallOnEndOverlap)
  (return false))

(fn StartInteract
  (Default|CallOnStartInteract)
  (return false))

(fn StartOverlap
  (Rendering|SetRenderCustomDepth (Variables|Default|GetComponent) true)
  (Default|CallOnStartOverlap)
  (return false))