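; BP_Turn is a trigger actor that smoothly turns the player 90 degrees in yaw when their capsule overlaps its box.
; The overlap sets the player's IsTurning flag, then a timeline lerps yaw to the target, printing each value, and clears the flag when finished.
; The construction script aims an arrow by the Direction setting, but the turn itself ignores Direction and always adds 90 degrees.
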(event OnComponentBeginOverlap(Box)
  (params (OverlappedComponent :type Primitive%20Component%20Object%20Reference) (OtherActor :type Actor%20Object%20Reference) (OtherComp :type Primitive%20Component%20Object%20Reference) (OtherBodyIndex :type Integer) (bFromSweep :type Boolean) (SweepResult :type Hit%20Result%20Structure%20%28by%20ref%29))
  (bind _returnvalue (Transformation|GetActorRotation OtherActor))
  (bind _asbp_player (Utilities|Casting|CastToBP_Player OtherActor))
  (if (== OtherComp (Variables|/Script/Engine.Character|GetCapsuleComponent _asbp_player))
    (Variables|/Game/Blueprint/BP_Player.BP_Player_C|SetIsTurning _asbp_player true)
    (bind _output_get (Variables|Default|SetCurRotate (.yaw (Transformation|GetActorRotation OtherActor))))
    (Variables|Default|SetTargetRotate (+ _output_get 9e+01))
    (bind _newtrack_0 (Timeline|RotateLerp PlayFromStart)
      (:Update
        (Transformation|SetActorRotation OtherActor (Math|Rotator|MakeRotator (.roll _returnvalue) (.pitch _returnvalue) (Math|Float|Lerp (Variables|Default|GetCurRotate) (Variables|Default|GetTargetRotate) _newtrack_0)))
        (Development|PrintString (Utilities|String|ToString(Float) (Math|Float|Lerp (Variables|Default|GetCurRotate) (Variables|Default|GetTargetRotate) _newtrack_0))))
      (:Finished
        (Variables|/Game/Blueprint/BP_Player.BP_Player_C|SetIsTurning _asbp_player false)))))

(event EventBeginPlay)

(event Collision|EventActorBeginOverlap
  (params (OtherActor :type Actor%20Object%20Reference)))

(event EventTick
  (params (DeltaSeconds :type Float%20%28single-precision%29)))

(fn ConstructionScript
  (Transformation|SetWorldRotation (Variables|Default|GetArrow) (Math|Rotator|MakeRotator 0.0 0.0 (Utilities|Select :Index (Variables|Default|GetDirection) :NewEnumerator0 0.0 :NewEnumerator1 1.8e+02 :NewEnumerator2 9e+01 :NewEnumerator3 2.7e+02)) false false))